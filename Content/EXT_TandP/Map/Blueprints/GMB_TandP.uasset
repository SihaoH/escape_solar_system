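; Game mode that spawns and orients the player after portal or teleporter travel between maps.
; ChoosePlayerStart picks the PlayerStart whose tag matches the game instance's ID and fires Loaded on the matching teleporter, otherwise falling back to the first start.
; On BeginPlay, portal arrivals get their saved camera rotation restored, offset by the matching portal's destination yaw, while teleport arrivals have their character mesh hidden briefly.
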(event `self.ReceiveBeginPlay`
  ;[0 0.1958 1] When the character is sent through the Portal, the "GMB" will adjust the rotation of the character's camera to maintain the previous rotation. When the character is sent by Teleportation, the "GMB" will set the Character's Mesh to be invisible for 1.6 seconds.
  (bind _asbc_game_instance (cast `/Game/EXT_TandP/Map/Blueprints/BC_GameInstance` (`GameplayStatics.GetGameInstance`)))
  (bind _asbp_character (cast `/Game/EXT_TandP/Demo/Character/BP_Character` (`GameplayStatics.GetPlayerCharacter` 0)))
  (if (`/Game/EXT_TandP/Map/Blueprints/BC_GameInstance.Portal` _asbc_game_instance)
    (bind _outactors (`GameplayStatics.GetAllActorsOfClass` "/Game/EXT_TandP/Portals/Versions/P-A-M/BP_Portal0.BP_Portal0_C"))
    (for _array_element _outactors
      (if (== (`/Game/EXT_TandP/Portals/Versions/P-A-M/BP_Portal0.Portal ID` _array_element) (`/Game/EXT_TandP/Map/Blueprints/BC_GameInstance.ID` _asbc_game_instance))
        (bind (_returnvalue_roll _returnvalue_pitch _returnvalue_yaw) (`KismetMathLibrary.BreakRotator` (`SceneComponent.K2_GetComponentRotation` (`/Game/EXT_TandP/Portals/Versions/P-A-M/BP_Portal0.SM_Destination Location` _array_element))))
        (`Controller.SetControlRotation` (`Pawn.GetController` _asbp_character) (`KismetMathLibrary.MakeRotator` (`/Game/EXT_TandP/Map/Blueprints/BC_GameInstance.Camera Rotation X` _asbc_game_instance) (`/Game/EXT_TandP/Map/Blueprints/BC_GameInstance.Camera Rotation Y` _asbc_game_instance) (+ (+ _returnvalue_yaw 90.0) (`/Game/EXT_TandP/Map/Blueprints/BC_GameInstance.Camera Rotation Z` _asbc_game_instance))))))
    (elif (`/Game/EXT_TandP/Map/Blueprints/BC_GameInstance.Teleport` _asbc_game_instance)
      (bind _mesh (`Character.Mesh` _asbp_character))
      (`SceneComponent.SetVisibility` _mesh false false)
      (`KismetSystemLibrary.Delay` 1.6)
      (`SceneComponent.SetVisibility` _mesh true false))))

(fn `ChoosePlayerStart`
  (params (Player :type "Controller Object Reference"))
  (returns (ReturnValue :type "Actor Object Reference"))
  ;[0.7195 0 1] If the character was sent to another map, the "Game Mode Base" is responsible when the map is being loaded to set the "PlayerStart" that will be used to spawn the character. When this happens, call custom event on "Teleportation" if needed.
  (bind _asbc_game_instance (cast `/Game/EXT_TandP/Map/Blueprints/BC_GameInstance` (`GameplayStatics.GetGameInstance`)))
  (bind _outactors (`GameplayStatics.GetAllActorsOfClass` "/Script/Engine.PlayerStart"))
  (for _array_element _outactors
    (if (== (`PlayerStart.PlayerStartTag` _array_element) (`/Game/EXT_TandP/Map/Blueprints/BC_GameInstance.ID` _asbc_game_instance))
      (set `self.Player Start` _array_element)
      (set `self.LevelTravelling` true)
      (bind _outactors_2 (`GameplayStatics.GetAllActorsOfClass` "/Game/EXT_TandP/Teleportations/Versions/T-A-M/BP_Teleportation0.BP_Teleportation0_C"))
      (for _array_element_2 _outactors_2
        (if (== (`/Game/EXT_TandP/Teleportations/Versions/T-A-M/BP_Teleportation0.Teleportation ID` _array_element_2) (`/Game/EXT_TandP/Map/Blueprints/BC_GameInstance.ID` _asbc_game_instance))
          (`/Game/EXT_TandP/Teleportations/Versions/T-A-M/BP_Teleportation0.Loaded` _array_element_2)
          (return _array_element)))))
  (if (`self.LevelTravelling`)
    (return (`self.Player Start`))
    (else
      (return (`|GetArrayItem` _outactors)))))

(fn `UserConstructionScript`)