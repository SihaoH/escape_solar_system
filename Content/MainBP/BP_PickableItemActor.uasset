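; BP_PickableItemActor is a world item that BP_MainCharacter can pick up, with debug prints for feedback.
; Its trigger overlaps set and clear the character's PickableActor reference.
; PickUp hides the actor, disables collision and returns ItemRowName with a random count.
; If that row exists in PickableItemDataTable, it sets a random-delay timer for Activate to restore the actor, though both random ranges are zero here.
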(event `self.PickupTrigger.OnComponentBeginOverlap`
  (params (OverlappedComponent :type "PrimitiveComponent Object Reference") (OtherActor :type "Actor Object Reference") (OtherComp :type "PrimitiveComponent Object Reference") (OtherBodyIndex :type Integer) (bFromSweep :type Boolean) (SweepResult :type "HitResult Structure (by ref)"))
  (bind _asbp_main_character (cast `/Game/MainBP/Blueprints/BP_MainCharacter` OtherActor))
  (set `/Game/MainBP/Blueprints/BP_MainCharacter.PickableActor` self _asbp_main_character)
  (`KismetSystemLibrary.PrintString` "可以拾取"))

(event `self.PickupTrigger.OnComponentEndOverlap`
  (params (OverlappedComponent :type "PrimitiveComponent Object Reference") (OtherActor :type "Actor Object Reference") (OtherComp :type "PrimitiveComponent Object Reference") (OtherBodyIndex :type Integer))
  (bind _asbp_main_character (cast `/Game/MainBP/Blueprints/BP_MainCharacter` OtherActor))
  (set `/Game/MainBP/Blueprints/BP_MainCharacter.PickableActor` null _asbp_main_character)
  (`KismetSystemLibrary.PrintString` "没有了"))

(fn `Activate`
  (`self.SetActorEnableCollision` true)
  (`self.SetActorHiddenInGame` false))

(fn `PickUp`
  (returns (RowName :type Name) (Count :type Integer))
  (bind _itemrowname (`self.ItemRowName`))
  (`self.SetActorEnableCollision` false)
  (`self.SetActorHiddenInGame` true)
  (`|GetDataTableRow` "/Game/Item/PickableItemDataTable.PickableItemDataTable" _itemrowname
    (:`then`
      (`KismetSystemLibrary.K2_SetTimer` null "Activate" (`KismetMathLibrary.RandomFloatInRange` 0.0)))
    (:`RowNotFound`
      (`KismetSystemLibrary.PrintString` "未在可拾取物品数据表中找到该物品")))
  (return _itemrowname (`KismetMathLibrary.RandomIntegerInRange` 0)))

(fn `UserConstructionScript`)