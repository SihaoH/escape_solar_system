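; BP_Planet is a planet actor that spins on its local yaw axis every tick at RotationVelocity scaled by delta time.
; BeginPlay caches its distance from the world origin as DistanceRadius, which only the disconnected orbit logic reads.
; Two unwired chains never run: inverse-square gravity messages to actors overlapping its Sphere, and a circular XY orbit around the origin using math expression nodes.
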(event `self.ReceiveBeginPlay`
  (set `self.DistanceRadius` (`KismetMathLibrary.Vector_Distance` (0.0 0.0 0.0) (`self.K2_GetActorLocation`))))

(event `self.ReceiveTick`
  (params (DeltaSeconds :type "Float (single-precision)"))
  (`|ExecutionSequence`
    (:`then_0`
      ;[1 1 1] 自转
      (`self.K2_AddActorLocalRotation` (`KismetMathLibrary.MakeRotator` 0.0 0.0 (* DeltaSeconds (`self.RotationVelocity`)))))))

(event `self.ReceiveActorBeginOverlap`
  (params (OtherActor :type "Actor Object Reference")))

(fn `UserConstructionScript`)