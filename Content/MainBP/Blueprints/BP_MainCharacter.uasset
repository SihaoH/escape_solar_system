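; Main character Blueprint that picks up nearby items into its Backpack.
; Capsule overlaps track the current pickable item actor, and pressing E picks it up, adds its row name and count to the Backpack, and prints the amount.
; Fall damage is unfinished: capsule hits compare speed relative to the hit actor against a threshold, but the branch is empty and the damage formula is unconnected.
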(event `self.CapsuleComponent.OnComponentHit`
  (params (HitComponent :type "PrimitiveComponent Object Reference") (OtherActor :type "Actor Object Reference") (OtherComp :type "PrimitiveComponent Object Reference") (NormalImpulse :type "Vector Structure") (Hit :type "HitResult Structure (by ref)"))
  ;[1 1 1] 跌落伤害：跌落速度超过1000，每100速度扣1点血；跌落时的速度需要减去星球的速度，即相对速度才能算是跌落速度
  (if (> (- (`KismetMathLibrary.VSize` (- (`SceneComponent.GetComponentVelocity` HitComponent) (`self.GetVelocity` OtherActor))) 1000.0) 0.0)
    _))

(event `Key|E`
  (params (Key :type "Key Structure"))
  (bind _pickableactor (`self.PickableActor`))
  (:`Pressed`
    (if (!= _pickableactor null)
      (bind (_rowname _count) (`/Game/MainBP/BP_PickableItemActor.PickUp` _pickableactor))
      (bind _returnvalue (`BackpackComponent.AddItem` (`self.Backpack`) _rowname _count))
      (`KismetSystemLibrary.PrintString` (`KismetStringLibrary.Concat_StrStr` "拾取了" (`KismetStringLibrary.Conv_IntToString` _returnvalue) "个")))))

(event `self.CapsuleComponent.OnComponentBeginOverlap`
  (params (OverlappedComponent :type "PrimitiveComponent Object Reference") (OtherActor :type "Actor Object Reference") (OtherComp :type "PrimitiveComponent Object Reference") (OtherBodyIndex :type Integer) (bFromSweep :type Boolean) (SweepResult :type "HitResult Structure (by ref)"))
  (bind _asbp_pickable_item_actor (cast `/Game/MainBP/BP_PickableItemActor` OtherActor))
  (set `self.PickableActor` _asbp_pickable_item_actor))

(event `self.CapsuleComponent.OnComponentEndOverlap`
  (params (OverlappedComponent :type "PrimitiveComponent Object Reference") (OtherActor :type "Actor Object Reference") (OtherComp :type "PrimitiveComponent Object Reference") (OtherBodyIndex :type Integer))
  (if (== OtherActor (`self.PickableActor`))
    (set `self.PickableActor` null)))

(fn `UserConstructionScript`)