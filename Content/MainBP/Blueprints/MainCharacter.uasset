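; MainCharacter is the player character Blueprint, with HP and MP, fall damage, and the ability to board a spaceship.
; BeginPlay fills current HP and MP from their maximums.
; Pressing F while near the ship hides the character, disables its collision and possesses the Spaceship pawn.
; Capsule hits subtract HP in steps for impact speed above a threshold, measured relative to the hit actor's velocity so moving planets are accounted for.
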(event `Key|F`
  (params (Key :type "Key Structure"))
  ;[1 1 1] 按F登上飞船：需要靠近飞船
  (:`Pressed`
    (if (`self.IsCloseShip`)
      (`self.SetActorHiddenInGame` true)
      (`self.SetActorEnableCollision` false)
      (`Controller.Possess` (`self.GetController`) (`self.Spaceship`)) ; Possess the UFO pawn
    )))

(event `self.ReceiveBeginPlay`
  ;[1 1 1] 初始化HP和MP
  (set `self.CurHP` (`self.MaxHP`))
  (set `self.CurMP` (`self.MaxMP`)))

(event `self.CapsuleComponent.OnComponentHit`
  (params (HitComponent :type "PrimitiveComponent Object Reference") (OtherActor :type "Actor Object Reference") (OtherComp :type "PrimitiveComponent Object Reference") (NormalImpulse :type "Vector Structure") (Hit :type "HitResult Structure (by ref)"))
  (bind _returnvalue (- (`KismetMathLibrary.VSize` (- (`SceneComponent.GetComponentVelocity` HitComponent) (`self.GetVelocity` OtherActor))) 1000.0))
  ;[1 1 1] 跌落伤害：跌落速度超过1000，每100速度扣1点血；跌落时的速度需要减去星球的速度，即相对速度才能算是跌落速度
  (if (> _returnvalue 0.0)
    (set `self.CurHP` (- (`self.CurHP`) (`KismetMathLibrary.Conv_IntToDouble` (`KismetMathLibrary.FFloor` (/ _returnvalue 100.0)))))))

(fn `UserConstructionScript`)